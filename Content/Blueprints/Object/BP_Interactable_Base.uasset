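; Base class for interactable objects that rotate when activated and can be checked into key-coded placement structures.
; On BeginPlay it loads its DT_ItemData row by display name, sets mesh physics and caches player and game mode.
; ActiveObject toggles forward or reverse timeline rotation, flags the player busy and signals BPMoveObject.
; ReplaceStart and ReplaceFinish toggle physics and register or remove key-code matches with the game mode; CheckCorrectInspect is an empty hook.
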(event `self.ReceiveBeginPlay`
  (`|ExecutionSequence`
    (:`then_0`
      (`self.SetItemDataStruct`))
    (:`then_1`
      (`self.SetObjectSetting`))
    (:`then_2`
      (bind _asbp_player (cast `/Game/Blueprints/Character/BP_Player` (`GameplayStatics.GetPlayerCharacter` 0)))
      (set `self.PlayerRef` _asbp_player)
      (bind _asbp_game_mode (cast `/Game/Blueprints/BP_GameMode` (`GameplayStatics.GetGameMode`)))
      (set `self.GamemodeRef` _asbp_game_mode))))

(event `Rotation`
  (params (RotateComponent :type "SceneComponent Object Reference") (StartRotation :type "Rotator Structure") (DestinationRotation :type "Rotator Structure"))
  (set `/Game/Blueprints/Character/BP_Player.bIsObjectActive` true (`self.PlayerRef`))
  (bind (_direction _newtrack_0) (`Timeline|Timeline` :!via `PlayFromStart` :!label _label)
    (:`Update`
      (`SceneComponent.K2_SetRelativeRotation` RotateComponent (`KismetMathLibrary.RLerp` StartRotation DestinationRotation _newtrack_0 true) false false))
    (:`Finished`
      (set `/Game/Blueprints/Character/BP_Player.bIsObjectActive` false (`self.PlayerRef`))
      (`self.CheckCorrectInspect`))))

(event `ReverseRotation`
  (params (RotateComponent :type "SceneComponent Object Reference") (StartRotation :type "Rotator Structure") (DestinationRotation :type "Rotator Structure"))
  (set `/Game/Blueprints/Character/BP_Player.bIsObjectActive` true (`self.PlayerRef`))
  (goto _label :!via `ReverseFromEnd`))

(fn `ActiveObject`
  (bind _acitveobjectcomponent (`self.AcitveObjectComponent`))
  (bind _bp_moveobject (`self.BP_MoveObject`))
  (bind _relativerotation (`SceneComponent.RelativeRotation` _acitveobjectcomponent))
  (bind _returnvalue (`KismetMathLibrary.MakeRotator` (+ (.roll (`SceneComponent.RelativeRotation` _acitveobjectcomponent)) (.roll (`.ToRotation_39_8EA135394532D18D09AAD980D890DA13` (break `/Game/Data/Struct/ST_ItemData` (`self.ItemData`))))) (+ (.pitch (`SceneComponent.RelativeRotation` _acitveobjectcomponent)) (.pitch (`.ToRotation_39_8EA135394532D18D09AAD980D890DA13` (break `/Game/Data/Struct/ST_ItemData` (`self.ItemData`))))) (+ (.yaw (`SceneComponent.RelativeRotation` _acitveobjectcomponent)) (.yaw (`.ToRotation_39_8EA135394532D18D09AAD980D890DA13` (break `/Game/Data/Struct/ST_ItemData` (`self.ItemData`)))))))
  (if (`/Game/Blueprints/Character/BP_Player.bIsObjectActive` (`self.PlayerRef`))
    _
    (elif (`self.IsReverse`)
      (`self.ReverseRotation` _acitveobjectcomponent _relativerotation _returnvalue)
      (set `self.IsReverse` false)
      (`/Game/Blueprints/StructObject/MoveObject/BP_MoveObjectBase.MoveOrRotation` _bp_moveobject true)
      (else
        (`self.Rotation` _acitveobjectcomponent _relativerotation _returnvalue)
        (set `self.IsReverse` true)
        (`/Game/Blueprints/StructObject/MoveObject/BP_MoveObjectBase.MoveOrRotation` _bp_moveobject false)))))

(fn `CheckCorrectInspect`)

(fn `GetIsFinish`
  (returns (IsFinish :type Boolean))
  (return (`self.bIsFinish`)))

(fn `ReplaceFinish`
  (`PrimitiveComponent.SetSimulatePhysics` (`self.StaticMesh`) true)
  (if (`self.bIsReplace`)
    (`/Game/Blueprints/BP_GameMode.RemoveCheckStructure` (`self.GamemodeRef`) (`KismetSystemLibrary.GetDisplayName` self))
    (set `self.bIsReplace` false)))

(fn `ReplaceStart`
  (params (Structure :type "/Game/Blueprints/StructObject/BP_StructObject_Base Object Reference"))
  (bind (_itemdata_itemname _itemdata_physics _itemdata_inspect _itemdata_active _itemdata_mesh _itemdata_keycode) (break `/Game/Data/Struct/ST_ItemData` (`self.ItemData`)))
  (`PrimitiveComponent.SetSimulatePhysics` (`self.StaticMesh`) false)
  (if (== (`/Game/Blueprints/StructObject/BP_StructObject_Base.KeyCode` (`local.Structure`)) _itemdata_keycode)
    (`/Game/Blueprints/BP_GameMode.CheckStructure` (`self.GamemodeRef`) (`local.Structure`) (`KismetSystemLibrary.GetDisplayName` self))
    (set `self.bIsReplace` true)))

(fn `SetItemDataStruct`
  (bind _returnvalue (`|GetDataTableRow` "/Game/Data/DataTable/DT_ItemData.DT_ItemData" (`KismetStringLibrary.Conv_StringToName` (`KismetSystemLibrary.GetDisplayName` self)))
    (:`then`
      (set `self.ItemData` _returnvalue))))

(fn `SetObjectSetting`
  (bind (_itemdata_itemname _itemdata_physics) (break `/Game/Data/Struct/ST_ItemData` (`self.ItemData`)))
  (`PrimitiveComponent.SetSimulatePhysics` (`self.StaticMesh`) _itemdata_physics))

(fn `UserConstructionScript`)