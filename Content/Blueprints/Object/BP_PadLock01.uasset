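; Inspectable combination padlock puzzle that opens a door when its three rotatable parts match the correct rotations in ItemData.
; CheckCorrectInspect compares each part to its target offset by the body mesh's rotation, testing the absolute value of the summed axis deltas.
; On success a timeline raises the metal pieces, then FinishPadLock ends inspection, calls MoveOrRotation on the BP_Door01 found at BeginPlay, and drops the lock with physics.
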(event `self.ReceiveBeginPlay`
  (`parent.ReceiveBeginPlay`)
  (bind _returnvalue (`GameplayStatics.GetActorOfClass` "/Game/Blueprints/StructObject/MoveObject/BP_Door01.BP_Door01_C"))
  (set `self.MoveActor` _returnvalue))

(event `UpMetalPieces`
  (params (CurrentLocation :type "Vector Structure") (DestinationLocation :type "Vector Structure"))
  (bind (_direction _newtrack_0) (`Timeline|Timeline_0`)
    (:`Update`
      (`SceneComponent.K2_SetWorldLocation` (`self.MetalPieces`) (`KismetMathLibrary.VLerp` CurrentLocation DestinationLocation _newtrack_0) false false))
    (:`Finished`
      (`self.FinishPadLock`))))

(fn `CheckCorrectInspect`
  (bind (_itemdata_itemname _itemdata_physics _itemdata_inspect _itemdata_active _itemdata_mesh _itemdata_keycode _itemdata_correctmesh _itemdata_inspectlocation _itemdata_inspectrotation _itemdata_torotation _itemdata_correctrotation) (break `/Game/Data/Struct/ST_ItemData` (`self.ItemData`)))
  (bind (_itemdata_itemname_2 _itemdata_physics_2 _itemdata_inspect_2 _itemdata_active_2 _itemdata_mesh_2 _itemdata_keycode_2 _itemdata_correctmesh_2 _itemdata_inspectlocation_2 _itemdata_inspectrotation_2 _itemdata_torotation_2 _itemdata_correctrotation_2) (break `/Game/Data/Struct/ST_ItemData` (`self.ItemData`)))
  (bind (_itemdata_itemname_3 _itemdata_physics_3 _itemdata_inspect_3 _itemdata_active_3 _itemdata_mesh_3 _itemdata_keycode_3 _itemdata_correctmesh_3 _itemdata_inspectlocation_3 _itemdata_inspectrotation_3 _itemdata_torotation_3 _itemdata_correctrotation_3) (break `/Game/Data/Struct/ST_ItemData` (`self.ItemData`)))
  (bind _returnvalue (`SceneComponent.K2_GetComponentLocation` (`self.MetalPieces`)))
  (`parent.CheckCorrectInspect`)
  (if (`self.CheckRotation` (`SceneComponent.RelativeRotation` (`self.Scene`)) (`|GetArrayItem` _itemdata_correctrotation_2))
    (if (`self.CheckRotation` (`SceneComponent.RelativeRotation` (`self.Scene1`)) (`|GetArrayItem` _itemdata_correctrotation_3 1))
      (if (`self.CheckRotation` (`SceneComponent.RelativeRotation` (`self.Scene2`)) (`|GetArrayItem` _itemdata_correctrotation 2))
        (`self.UpMetalPieces` _returnvalue (+ _returnvalue (0.0 0.0 10.0)))))))

(fn `CheckRotation`
  (params (CurrentRotation :type "Rotator Structure") (DestinationRotation :type "Rotator Structure"))
  (returns (IsCorrect :type Boolean))
  (bind (_relativerotation_roll _relativerotation_pitch _relativerotation_yaw) (`KismetMathLibrary.BreakRotator` (`SceneComponent.RelativeRotation` (`self.StaticMesh`))))
  (bind (_returnvalue_roll _returnvalue_pitch _returnvalue_yaw) (`KismetMathLibrary.BreakRotator` (`KismetMathLibrary.NormalizedDeltaRotator` CurrentRotation (`KismetMathLibrary.MakeRotator` (+ _relativerotation_roll (.roll DestinationRotation)) (+ _relativerotation_pitch (.pitch DestinationRotation)) (+ _relativerotation_yaw (.yaw DestinationRotation))))))
  (return (< (`KismetMathLibrary.Abs` (+ _returnvalue_roll _returnvalue_pitch _returnvalue_yaw)) 1.0)))

(fn `FinishPadLock`
  (`/Game/Blueprints/Character/BP_Player.DirectInspectFinish` (`self.PlayerRef`))
  (`/Game/Blueprints/StructObject/MoveObject/BP_MoveObjectBase.MoveOrRotation` (`self.MoveActor`) false)
  (`PrimitiveComponent.SetSimulatePhysics` (`self.StaticMesh`) true)
  (set `self.bIsFinish` true))

(fn `UserConstructionScript`
  (`parent.UserConstructionScript`))