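; BP_Box01 is a box object that animates a 90-degree pitch rotation of its Scene component when CheckCorrectInspect runs.
; The CheckCorrectInspect override calls its parent, then passes the current relative rotation and the pitched target to the Rotate event.
; Rotate plays a timeline from the start, using its track as the alpha to lerp the component's relative rotation between the two.
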(event `Rotate`
  (params (StartRotation :type "Rotator Structure") (FinishRotation :type "Rotator Structure"))
  (bind (_direction _newtrack_0) (`Timeline|Timeline_0` :!via `PlayFromStart`)
    (:`Update`
      (`SceneComponent.K2_SetRelativeRotation` (`self.Scene`) (`KismetMathLibrary.RLerp` StartRotation FinishRotation _newtrack_0) false false))))

(fn `CheckCorrectInspect`
  (bind _relativerotation (`SceneComponent.RelativeRotation` (`self.Scene`)))
  (`parent.CheckCorrectInspect`)
  (`self.Rotate` _relativerotation (`KismetMathLibrary.MakeRotator` (.roll _relativerotation) (+ (.pitch _relativerotation) 90.0) (.yaw _relativerotation))))

(fn `UserConstructionScript`
  (`parent.UserConstructionScript`))