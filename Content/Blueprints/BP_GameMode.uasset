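; Game mode that coordinates key-code item puzzles and switches the player between main and inspection UI.
; On BeginPlay it creates both widgets and binds to BP_Player's check events.
; Matching key codes raise a per-structure count and record the grabbed item, triggering MoveOrRotation once the required count is met; CheckOutStructure reverses an item's contribution.
; Helper functions swap the widgets and toggle cursor input for direct inspection.
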(event `self.ReceiveBeginPlay`
  (bind _returnvalue (`|CreateWidget` "/Game/UI/WBP_MainUI.WBP_MainUI_C"))
  (bind _output_get (set `self.MainUI` _returnvalue))
  (`UserWidget.AddToViewport` _output_get 0)
  (bind _returnvalue_2 (`|CreateWidget` "/Game/UI/WBP_InspectItem.WBP_InspectItem_C"))
  (set `self.InspectUI` _returnvalue_2)
  (set `self.PlayerController` (`GameplayStatics.GetPlayerController` 0))
  (bind _asbp_player (cast `/Game/Blueprints/Character/BP_Player` (`GameplayStatics.GetPlayerPawn` 0)))
  (bind _output_get_2 (set `self.BP_Player` _asbp_player))
  (add `/Game/Blueprints/Character/BP_Player.CorrectCheck` _output_get_2 (delegate `CorrectCheck`))
  (add `/Game/Blueprints/Character/BP_Player.OutStructure` _output_get_2 (`|CreateDelegate` :!event `CheckOutStructure`)))

(event `CorrectCheck`
  (params (Structure :type "/Game/Blueprints/StructObject/BP_StructObject_Base Object Reference") (KeyCode :type Integer) (GrabItemName :type String))
  (bind (_structdata_objectname _structdata_mesh _structdata_correctrotation _structdata_codecount) (break `/Game/Data/Struct/ST_StructObject` (`/Game/Blueprints/StructObject/BP_StructObject_Base.StructData` Structure)))
  (bind _sturcturecheck (`self.SturctureCheck`))
  (bind _returnvalue (+ (`BlueprintMapLibrary.Map_Find` _sturcturecheck _structdata_objectname) 1))
  (if (== KeyCode (`/Game/Blueprints/StructObject/BP_StructObject_Base.KeyCode` Structure))
    (`BlueprintMapLibrary.Map_Add` _sturcturecheck _structdata_objectname _returnvalue)
    (`BlueprintMapLibrary.Map_Add` (`self.ObjectAndStructure`) GrabItemName _structdata_objectname)
    (if (> _returnvalue _structdata_codecount)
      (`/Game/Blueprints/StructObject/MoveObject/BP_MoveObjectBase.MoveOrRotation` (`/Game/Blueprints/StructObject/BP_StructObject_Base.BP_MoveObjectBase` Structure)))))

(fn `CheckOutStructure`
  (params (GrabItemName :type String))
  (bind _sturcturecheck (`self.SturctureCheck`))
  (bind (_value _returnvalue) (`BlueprintMapLibrary.Map_Find` (`self.ObjectAndStructure`) GrabItemName))
  (if _returnvalue
    (`BlueprintMapLibrary.Map_Add` _sturcturecheck _value (- (`BlueprintMapLibrary.Map_Find` _sturcturecheck _value) 1))
    (`BlueprintMapLibrary.Map_Remove` (`self.ObjectAndStructure`) (`local.GrabItemName`))))

(fn `DirectInspectFinish`
  (bind _playercontroller (`self.PlayerController`))
  (`WidgetBlueprintLibrary.SetInputMode_GameOnly` _playercontroller)
  (set `PlayerController.bShowMouseCursor` false _playercontroller))

(fn `DirectInspectStart`
  (bind _playercontroller (`self.PlayerController`))
  (`WidgetBlueprintLibrary.SetInputMode_GameAndUIEx` _playercontroller (`self.MainUI`) "LockAlways")
  (set `PlayerController.bShowMouseCursor` true _playercontroller))

(fn `InspectFinish`
  (`Widget.RemoveFromParent` (`self.InspectUI`))
  (`UserWidget.AddToViewport` (`self.MainUI`) 0))

(fn `InspectStart`
  (`UserWidget.AddToViewport` (`self.InspectUI`) 0)
  (`Widget.RemoveFromParent` (`self.MainUI`)))

(fn `UserConstructionScript`)