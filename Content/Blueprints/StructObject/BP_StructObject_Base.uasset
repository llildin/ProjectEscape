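; BP_StructObject_Base is a base Blueprint for structure objects that configures itself from data at BeginPlay.
; It first looks up its row in DT_StructObject, using its own display name as the row name, and stores the result in StructData.
; It then applies the row's mesh to StaticMesh and shifts CheckMesh by the row's CorrectLocation as a local offset.
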(event `self.ReceiveBeginPlay`
  (`|ExecutionSequence`
    (:`then_0`
      (`self.SetObjectDataStruct`))
    (:`then_1`
      (`self.SetStructSetting`))))

(fn `SetObjectDataStruct`
  (bind _returnvalue (`|GetDataTableRow` "/Game/Data/DataTable/DT_StructObject.DT_StructObject" (`KismetStringLibrary.Conv_StringToName` (`KismetSystemLibrary.GetDisplayName` self)))
    (:`then`
      (set `self.StructData` _returnvalue))))

(fn `SetStructSetting`
  (bind (_structdata_objectname _structdata_mesh _structdata_correctlocation) (break `/Game/Data/Struct/ST_StructObject` (`self.StructData`)))
  (`StaticMeshComponent.SetStaticMesh` (`self.StaticMesh`) _structdata_mesh)
  (`SceneComponent.K2_AddLocalOffset` (`self.CheckMesh`) _structdata_correctlocation false false))

(fn `UserConstructionScript`)