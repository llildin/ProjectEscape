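; Base actor for data-driven moving objects that slide or rotate a MoveMesh component forward or back.
; On BeginPlay it loads StructData from the DT_MoveObject row whose name matches the actor's display name.
; MoveOrRotation uses the row's IsMove flag to pick Move or Rotate.
; Each drives its own timeline, played or reversed, lerping relative location or rotation from zero to the row's offset.
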(event `self.ReceiveBeginPlay`
  (`self.SetMoveObjectStruct`))

(event `Rotate`
  (params (IsReverse :type Boolean))
  (bind (_structdata_objectname _structdata_movemesh _structdata_addlocation _structdata_addrotation) (break `/Game/Data/Struct/ST_MoveObject` (`self.StructData`)))
  (if IsReverse
    (bind (_direction _newtrack_0) (`Timeline|Timeline` :!via `Reverse` :!label _label)
      (:`Update`
        (`SceneComponent.K2_SetRelativeRotation` (`self.MoveMesh`) (`KismetMathLibrary.RLerp` (struct) _structdata_addrotation _newtrack_0) false false)))
    (else
      (goto _label))))

(event `Move`
  (params (IsReverse :type Boolean))
  (bind (_structdata_objectname _structdata_movemesh _structdata_addlocation) (break `/Game/Data/Struct/ST_MoveObject` (`self.StructData`)))
  (if IsReverse
    (bind (_direction _newtrack_0) (`Timeline|Timeline_0` :!via `Reverse` :!label _label_2)
      (:`Update`
        (`SceneComponent.K2_SetRelativeLocation` (`self.MoveMesh`) (`KismetMathLibrary.VLerp` (0.0 0.0 0.0) _structdata_addlocation _newtrack_0) false false)))
    (else
      (goto _label_2))))

(fn `MoveOrRotation`
  (params (IsReverse :type Boolean))
  (bind (_structdata_objectname _structdata_movemesh _structdata_addlocation _structdata_addrotation _structdata_ismove) (break `/Game/Data/Struct/ST_MoveObject` (`self.StructData`)))
  (if _structdata_ismove
    (`self.Move` IsReverse)
    (else
      (`self.Rotate` IsReverse))))

(fn `SetMoveObjectStruct`
  (bind _returnvalue (`|GetDataTableRow` "/Game/Data/DataTable/DT_MoveObject.DT_MoveObject" (`KismetStringLibrary.Conv_StringToName` (`KismetSystemLibrary.GetDisplayName` self)))
    (:`then`
      (set `self.StructData` _returnvalue))))

(fn `UserConstructionScript`)