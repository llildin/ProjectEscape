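; Player controller that translates input into actions on the cached BP_Player character: moving, looking, jumping, and grabbing, collecting, selecting and inspecting items.
; On BeginPlay it caches the character, and handlers gate most inputs on its grab, inspect and direct-inspect flags.
; While inspecting an item, movement is blocked and look axes rotate the item only while Select is held.
; CheckItem toggles held-item inspection when grabbing, otherwise direct inspection.
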(event `InputAxis|Turn`
  (params (AxisValue :type "Float (single-precision)"))
  (bind _bp_player (`self.BP_Player`))
  (if (`/Game/Blueprints/Character/BP_Player.bIsDirectInspect` (`self.BP_Player`))
    _
    (elif (`/Game/Blueprints/Character/BP_Player.bIsInspectItem` _bp_player)
      (if (`self.bIsClick`)
        (`/Game/Blueprints/Character/BP_Player.TurnItem` (`self.BP_Player`) AxisValue))
      (else
        (`/Game/Blueprints/Character/BP_Player.Turn` _bp_player AxisValue)))))

(event `self.ReceiveBeginPlay`
  (bind _asbp_player (cast `/Game/Blueprints/Character/BP_Player` (`GameplayStatics.GetPlayerCharacter` 0)))
  (set `self.BP_Player` _asbp_player))

(event `InputAxis|LookUp`
  (params (AxisValue :type "Float (single-precision)"))
  (bind _bp_player (`self.BP_Player`))
  (if (`/Game/Blueprints/Character/BP_Player.bIsDirectInspect` (`self.BP_Player`))
    _
    (elif (`/Game/Blueprints/Character/BP_Player.bIsInspectItem` _bp_player)
      (if (`self.bIsClick`)
        (`/Game/Blueprints/Character/BP_Player.LookUpItem` (`self.BP_Player`) AxisValue))
      (else
        (`/Game/Blueprints/Character/BP_Player.LookUp` _bp_player AxisValue)))))

(event `InputAxis|MoveForward`
  (params (AxisValue :type "Float (single-precision)"))
  (bind _bp_player (`self.BP_Player`))
  ; Move
  (if (not (`/Game/Blueprints/Character/BP_Player.bIsInspectItem` _bp_player))
    (`/Game/Blueprints/Character/BP_Player.Move` _bp_player true AxisValue)))

(event `InputAction|Jump`
  (params (Key :type "Key Structure"))
  (:`Pressed`
    (`Character.Jump` (`self.BP_Player`))))

(event `InputAxis|MoveRight`
  (params (AxisValue :type "Float (single-precision)"))
  (bind _bp_player (`self.BP_Player`))
  ; Move
  (if (not (`/Game/Blueprints/Character/BP_Player.bIsInspectItem` _bp_player))
    (`/Game/Blueprints/Character/BP_Player.Move` _bp_player false AxisValue)))

(event `InputAction|Select`
  (params (Key :type "Key Structure"))
  (bind _bp_player (`self.BP_Player`))
  (:`Pressed`
    (set `self.bIsClick` true)
    (if (`/Game/Blueprints/Character/BP_Player.bIsGrab` _bp_player)
      (if (not (`/Game/Blueprints/Character/BP_Player.bIsInspectItem` (`self.BP_Player`)))
        (`/Game/Blueprints/Character/BP_Player.ReplaceItem` _bp_player))
      (else
        (`/Game/Blueprints/Character/BP_Player.GrabItemStart` _bp_player))))
  (:`Released`
    (set `self.bIsClick` false)))

(event `InputAction|Select`
  (params (Key :type "Key Structure"))
  (bind _bp_player (`self.BP_Player`))
  (bind _bp_player_2 (`self.BP_Player`))
  (:`Pressed`
    (if (`/Game/Blueprints/Character/BP_Player.bIsDirectInspect` _bp_player)
      (`/Game/Blueprints/Character/BP_Player.DirectInspectRotation` _bp_player_2)
      (elif (`/Game/Blueprints/Character/BP_Player.bIsInspectItem` _bp_player)
        (`/Game/Blueprints/Character/BP_Player.InspectItemClick` _bp_player_2)))))

(event `InputAction|Cancel`
  (params (Key :type "Key Structure"))
  (:`Pressed`
    (if (`/Game/Blueprints/Character/BP_Player.bIsGrab` (`self.BP_Player`))
      (if (not (`/Game/Blueprints/Character/BP_Player.bIsInspectItem` (`self.BP_Player`)))
        (`/Game/Blueprints/Character/BP_Player.GrabItemFinish` (`self.BP_Player`))))))

(event `InputAction|RightItem`
  (params (Key :type "Key Structure"))
  (bind _bp_player (`self.BP_Player`))
  (:`Pressed`
    (if (`/Game/Blueprints/Character/BP_Player.bIsDirectInspect` _bp_player)
      _
      (elif (not (`/Game/Blueprints/Character/BP_Player.bIsInspectItem` _bp_player))
        (`/Game/Blueprints/Character/BP_Player.RightItemSelect` _bp_player)))))

(event `InputAction|CheckItem`
  (params (Key :type "Key Structure"))
  (bind _bp_player (`self.BP_Player`))
  (bind _bp_player_2 (`self.BP_Player`))
  (bind _bp_player_3 (`self.BP_Player`))
  (bind _bisinspectitem (`/Game/Blueprints/Character/BP_Player.bIsInspectItem` _bp_player))
  (:`Pressed`
    (if (`/Game/Blueprints/Character/BP_Player.bIsGrab` _bp_player)
      (if _bisinspectitem
        (`/Game/Blueprints/Character/BP_Player.InspectItemFinish` _bp_player_2)
        (else
          (`/Game/Blueprints/Character/BP_Player.InspectItemStart` _bp_player_2)))
      (elif _bisinspectitem
        (`/Game/Blueprints/Character/BP_Player.DirectInspectFinish` _bp_player_3)
        (else
          (`/Game/Blueprints/Character/BP_Player.DirectInspectStart` _bp_player_3))))))

(event `InputAction|LeftItem`
  (params (Key :type "Key Structure"))
  (bind _bp_player (`self.BP_Player`))
  (:`Pressed`
    (if (`/Game/Blueprints/Character/BP_Player.bIsDirectInspect` _bp_player)
      _
      (elif (not (`/Game/Blueprints/Character/BP_Player.bIsInspectItem` _bp_player))
        (`/Game/Blueprints/Character/BP_Player.LeftItemSelect` _bp_player)))))

(event `InputAction|GetItem`
  (params (Key :type "Key Structure"))
  (bind _bp_player (`self.BP_Player`))
  (:`Pressed`
    (if (`/Game/Blueprints/Character/BP_Player.bIsDirectInspect` _bp_player)
      _
      (elif (`/Game/Blueprints/Character/BP_Player.bIsInspectItem` _bp_player)
        _
        (elif (not (`/Game/Blueprints/Character/BP_Player.bIsGrab` _bp_player))
          (`/Game/Blueprints/Character/BP_Player.GetItem` _bp_player))))))

(fn `UserConstructionScript`)